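; Grass system actor that builds randomized triangle-blade grass as procedural mesh sections over traced ground.
; GenerateGrassTiles queues a grid of tile origins around the actor, then GenerateNextTile builds only the first pending one.
; Each tile line-traces a density-based grid, adding a double-sided triangle with varied position, height and width per hit.
; CheckLayer only prints the landscape grass paint weight; its threshold branch is unconnected, so it filters nothing.
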(event `GenerateGrassTiles`
  (bind (_returnvalue_x _returnvalue_y) (break `IntPoint` (/ (`self.GrassTileCount`) (make `IntPoint` 2 2))))
  (set `self.GrassMeshSectionIndex` 0)
  (`ProceduralMeshComponent.ClearAllMeshSections` (`self.GrassMesh`))
  (for _index (range (* _returnvalue_y -1) (+ _returnvalue_y 1))
    (for _index_2 (range (* _returnvalue_x -1) (+ _returnvalue_x 1))
      (`BlueprintMapLibrary.Map_Add` (`self.QueuedTiles`) (+ (* (`KismetMathLibrary.MakeVector` (`KismetMathLibrary.Conv_IntToDouble` _index_2) (`KismetMathLibrary.Conv_IntToDouble` _index)) (`self.TileSize`)) (`self.K2_GetActorLocation`)) -1)))
  (`self.GenerateNextTile`))

(event `ClearGrassTiles`
  (set `self.GrassMeshSectionIndex` 0)
  (`ProceduralMeshComponent.ClearAllMeshSections` (`self.GrassMesh`))
  (`BlueprintMapLibrary.Map_Clear` (`self.QueuedTiles`)))

(fn `GenerateGrassTile`
  (params (Origin :type "Vector Structure"))
  (locals (Gap :type "Float (double-precision)" :default 0.0) (Vertices :type "Array of Vector Structure") (VertexCount :type Integer) (Triangles :type "Array of Integer") (BaseVertex :type "Vector Structure") (UVs :type "Array of Vector2D Structure"))
  (bind _grassheightvariation (`self.GrassHeightVariation`))
  (bind _vertices (`local.Vertices`))
  (bind _grasswidth (`self.GrassWidth`))
  (bind _locationoffsetvariation (`self.LocationOffsetVariation`))
  (bind _uvs (`local.UVs`))
  (bind _triangles (`local.Triangles`))
  (bind _triangles_2 (`local.Triangles`))
  (bind _vertexcount (`local.VertexCount`))
  (bind _grassmeshsectionindex (`self.GrassMeshSectionIndex`))
  (bind _grassmesh (`self.GrassMesh`))
  (bind _returnvalue (* _grasswidth -1.0))
  (bind _returnvalue_2 (* _locationoffsetvariation -1.0))
  (bind _returnvalue_3 (+ _vertexcount 2))
  (bind _returnvalue_4 (+ _vertexcount 1))
  (bind _returnvalue_5 (/ (`self.GrassDensity`) 2.0))
  (bind _returnvalue_6 (`KismetMathLibrary.FTrunc` _returnvalue_5))
  (bind _returnvalue_7 (`KismetMathLibrary.FTrunc` (* _returnvalue_5 -1.0)))
  (set `local.Gap` (/ (`self.TileSize`) (`self.GrassDensity`)))
  (for _index (range _returnvalue_7 (+ _returnvalue_6 1))
    (for _index_2 (range _returnvalue_7 (+ _returnvalue_6 1))
      (bind _returnvalue_8 (+ (* (`KismetMathLibrary.MakeVector` (`KismetMathLibrary.Conv_IntToDouble` _index_2) (`KismetMathLibrary.Conv_IntToDouble` _index)) (`local.Gap`)) (`local.Origin`)))
      (bind (_outhit _returnvalue_9) (`KismetSystemLibrary.LineTraceSingle` (+ _returnvalue_8 (0.0 0.0 2000.0)) (+ _returnvalue_8 (0.0 0.0 -2000.0)) "TraceTypeQuery1"))
      (if _returnvalue_9
        (bind (_bblockinghit _binitialoverlap _time _distance _location) (`GameplayStatics.BreakHitResult` _outhit))
        (bind _returnvalue_10 (`LandscapeComponent.EditorGetPaintLayerWeightAtLocation` (`self.GetComponentByClass` (`self.Landscape`) "/Script/Landscape.LandscapeComponent") _location "/Game/ThirdPerson/Maps/ThirdPersonMap_sharedassets/grass_LayerInfo.grass_LayerInfo"))
        (`KismetSystemLibrary.PrintString` (`KismetStringLibrary.Conv_DoubleToString` _returnvalue_10))
        (bind _output_get (set `local.BaseVertex` (- _location (`self.K2_GetActorLocation`) (`KismetMathLibrary.MakeVector` (`KismetMathLibrary.RandomFloatInRange` _returnvalue_2 _locationoffsetvariation) (`KismetMathLibrary.RandomFloatInRange` _returnvalue_2 _locationoffsetvariation) 10.0))))
        (`KismetArrayLibrary.Array_Add` _vertices _output_get)
        (`KismetArrayLibrary.Array_Add` _vertices (+ _output_get (`KismetMathLibrary.MakeVector` 0.0 0.0 (+ (`self.GrassHeight`) (`KismetMathLibrary.RandomFloatInRange` (* _grassheightvariation -1.0) _grassheightvariation)))))
        (`KismetArrayLibrary.Array_Add` _vertices (+ _output_get (`KismetMathLibrary.MakeVector` (`KismetMathLibrary.RandomFloatInRange` _returnvalue _grasswidth) (`KismetMathLibrary.RandomFloatInRange` _returnvalue _grasswidth))))
        (`KismetArrayLibrary.Array_Add` _uvs)
        (`KismetArrayLibrary.Array_Add` _uvs (0.5 1.0))
        (`KismetArrayLibrary.Array_Add` _uvs (1.0 0.0))
        (`KismetArrayLibrary.Array_Add` _triangles _vertexcount)
        (`KismetArrayLibrary.Array_Add` _triangles _returnvalue_4)
        (`KismetArrayLibrary.Array_Add` _triangles _returnvalue_3)
        (`KismetArrayLibrary.Array_Add` _triangles_2 _vertexcount)
        (`KismetArrayLibrary.Array_Add` _triangles_2 _returnvalue_3)
        (`KismetArrayLibrary.Array_Add` _triangles_2 _returnvalue_4)
        (set `local.VertexCount` (+ (`local.VertexCount`) 3)))))
  (`ProceduralMeshComponent.CreateMeshSection_LinearColor` :`self` _grassmesh :`SectionIndex` _grassmeshsectionindex :`Vertices` (`local.Vertices`) :`Triangles` (`local.Triangles`) :`UV0` (`local.UVs`))
  (`PrimitiveComponent.SetMaterial` _grassmesh _grassmeshsectionindex "/Game/CLM_GrassSystem/Material/M_Grass.M_Grass")
  (`/Engine/EditorBlueprintResources/StandardMacros.IncrementInt` (`self.GrassMeshSectionIndex`)))

(fn `GenerateNextTile`
  (bind _values (`BlueprintMapLibrary.Map_Values` (`self.QueuedTiles`)))
  (for (_array_element _array_index) _values
    (if (== _array_element -1)
      (`|ExecutionSequence`
        (:`then_0`
          (break))
        (:`then_1`
          (bind _keys (`BlueprintMapLibrary.Map_Keys` (`self.QueuedTiles`)))
          (bind _output (`|GetArrayItem` _keys _array_index))
          (`BlueprintMapLibrary.Map_Add` (`self.QueuedTiles`) _output (`self.GrassMeshSectionIndex`))
          (`self.GenerateGrassTile` _output))))))

(fn `UserConstructionScript`)